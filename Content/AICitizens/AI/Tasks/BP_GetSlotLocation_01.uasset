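; Behavior tree task that picks a random reachable spot inside an AI citizen's assigned POI slot and writes it to the TargetLocation blackboard key.
; It offsets the slot box's world location by random X and Y within its rotated extent, with Z fixed at zero.
; A random reachable navmesh point near that position becomes the target.
; The task fails only when the blackboard POISlot is not a BP_BasePOISlot_01.
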(event `self.ReceiveExecute`
  (params (OwnerActor :type "Actor Object Reference"))
  ;[1 1 1] Select random reachable point in POI Slot bounding box
  (bind _asbp_base_poislot_01 (cast `/Game/AICitizens/Blueprints/BP_BasePOISlot_01` (`BTFunctionLibrary.GetBlackboardValueAsObject` (`self.POISlot`)))
    (:`then`
      (bind _box (`/Game/AICitizens/Blueprints/BP_BasePOISlot_01.Box` _asbp_base_poislot_01))
      (bind (_returnvalue_x _returnvalue_y) (`KismetMathLibrary.BreakVector` (`SceneComponent.K2_GetComponentLocation` _box)))
      (bind _x (.x (`KismetMathLibrary.GreaterGreater_VectorRotator` (`BoxComponent.GetScaledBoxExtent` _box) (`SceneComponent.K2_GetComponentRotation` _box))))
      (bind _y (.y (`KismetMathLibrary.GreaterGreater_VectorRotator` (`BoxComponent.GetScaledBoxExtent` _box) (`SceneComponent.K2_GetComponentRotation` _box))))
      (`BTFunctionLibrary.SetBlackboardValueAsVector` (`self.TargetLocation`) (`NavigationSystem.GetRandomReachablePointInRadius` (`KismetMathLibrary.MakeVector` (+ _returnvalue_x (`KismetMathLibrary.RandomFloatInRange` (* -1 _x) _x)) (+ _returnvalue_y (`KismetMathLibrary.RandomFloatInRange` (* -1 _y) _y))) 90.0))
      (`self.FinishExecute` true))
    (:`CastFailed`
      (`self.FinishExecute` false))))