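; Behavior tree task that turns an AI citizen to face the point of interest (BP_BasePOI_01) stored in its blackboard.
; Each AI tick it eases only the pawn's yaw toward the look-at angle with a float FInterpTo, then normalizes it.
; It succeeds once yaw is within a small tolerance of the target, and fails if the pawn or POI cast is invalid.
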(event `self.ReceiveTickAI`
  (params (OwnerController :type "AIController Object Reference") (ControlledPawn :type "Pawn Object Reference") (DeltaSeconds :type "Float (single-precision)"))
  (bind (_returnvalue_roll _returnvalue_pitch _returnvalue_yaw) (`KismetMathLibrary.BreakRotator` (`Actor.K2_GetActorRotation` ControlledPawn)))
  ;[1 1 1] Rotate AI character to POI
  (`/Engine/EditorBlueprintResources/StandardMacros.IsValid` ControlledPawn
    (:`Is Valid`
      (bind _asbp_base_poi_01 (cast `/Game/AICitizens/Blueprints/BP_BasePOI_01` (`BTFunctionLibrary.GetBlackboardValueAsObject` (`self.POI`)))
        (:`then`
          (bind (_returnvalue_roll_2 _returnvalue_pitch_2 _returnvalue_yaw_2) (`KismetMathLibrary.BreakRotator` (`KismetMathLibrary.FindLookAtRotation` (`Actor.K2_GetActorLocation` ControlledPawn) (`Actor.K2_GetActorLocation` _asbp_base_poi_01))))
          (bind _returnvalue (`KismetMathLibrary.NormalizeAxis` (`KismetMathLibrary.FInterpTo` _returnvalue_yaw _returnvalue_yaw_2 DeltaSeconds 5.0)))
          (`Actor.K2_SetActorRotation` ControlledPawn (`KismetMathLibrary.MakeRotator` _returnvalue_roll _returnvalue_pitch _returnvalue) false)
          (if (`KismetMathLibrary.NearlyEqual_FloatFloat` _returnvalue _returnvalue_yaw_2 1.0)
            (`self.FinishExecute` true)))
        (:`CastFailed`
          (`self.FinishExecute` false :!label _label))))
    (:`Is Not Valid`
      (`KismetSystemLibrary.PrintString` "AI Character is not valid" true true (struct :`R` 1.0 :`A` 1.0) 10.0)
      (goto _label))))