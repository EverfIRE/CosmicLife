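; Behavior tree task that makes an AI citizen play the animation assigned to its point-of-interest slot.
; On execute, it reads the POI slot from the Blackboard and passes that slot's animation to the controlled citizen character, failing if the citizen, slot or animation is invalid.
; It polls the character each AI tick and finishes successfully once the slot animation stops playing.
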(event `self.ReceiveExecute`
  (params (OwnerActor :type "Actor Object Reference"))
  ;[1 1 1] Play animation from POI Slot
  (bind _asaicontroller (cast `AIController` OwnerActor))
  (bind _asbp_base_aicitizen_character_01 (cast `/Game/AICitizens/AI/BP_BaseAICitizenCharacter_01` (`Controller.K2_GetPawn` _asaicontroller))
    (:`then`
      (bind _asbp_base_poislot_01 (cast `/Game/AICitizens/Blueprints/BP_BasePOISlot_01` (`BTFunctionLibrary.GetBlackboardValueAsObject` (`self.POISlot`)))
        (:`then`
          (bind _animation (`/Game/AICitizens/Blueprints/BP_BasePOISlot_01.GetAnimation` _asbp_base_poislot_01))
          (`/Engine/EditorBlueprintResources/StandardMacros.IsValid` _animation
            (:`Is Valid`
              (`/Game/AICitizens/AI/BP_BaseAICitizenCharacter_01.PlaySlotAnimation` _asbp_base_aicitizen_character_01 _animation))
            (:`Is Not Valid`
              (`self.FinishExecute` false))))
        (:`CastFailed`
          (`self.FinishExecute` false))))
    (:`CastFailed`
      (`self.FinishExecute` false))))

(event `self.ReceiveTickAI`
  (params (OwnerController :type "AIController Object Reference") (ControlledPawn :type "Pawn Object Reference") (DeltaSeconds :type "Float (single-precision)"))
  ;[1 1 1] Finish task when animation is finished
  (bind _asbp_base_aicitizen_character_01 (cast `/Game/AICitizens/AI/BP_BaseAICitizenCharacter_01` ControlledPawn)
    (:`then`
      (if (not (`/Game/AICitizens/AI/BP_BaseAICitizenCharacter_01.IsPlayingSlotAnimation` _asbp_base_aicitizen_character_01))
        (`self.FinishExecute` true)))
    (:`CastFailed`
      (`self.FinishExecute` false))))