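; Behavior Tree task for citizen AI that picks a random unoccupied slot at the blackboard's point of interest.
; It collects free slot actors from the POI's child actor components, writes one to the POISlot key and sets OccupiedBy to the owner.
; The random pick is re-rolled for validation, storing and claiming, so these can hit different slots, and its range skips the last entry.
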(event `self.ReceiveExecute`
  (params (OwnerActor :type "Actor Object Reference"))
  (bind _validslots (`self.ValidSlots`))
  (bind _item (`KismetArrayLibrary.Array_Get` _validslots (`KismetMathLibrary.RandomInteger` (- (`KismetArrayLibrary.Array_Length` _validslots) 1))))
  ;[1 1 1] Find all valid slots
  (`KismetArrayLibrary.Array_Clear` (`self.ValidSlots`))
  (bind _asbp_base_poi_01 (cast `/Game/AICitizens/Blueprints/BP_BasePOI_01` (`BTFunctionLibrary.GetBlackboardValueAsObject` (`self.POI`)))
    (:`then`
      (for _array_element (`Actor.K2_GetComponentsByClass` _asbp_base_poi_01 "/Script/Engine.ChildActorComponent")
        (bind _asbp_base_poislot_01 (cast `/Game/AICitizens/Blueprints/BP_BasePOISlot_01` (`ChildActorComponent.ChildActor` _array_element)))
        (if (not (`/Game/AICitizens/Blueprints/BP_BasePOISlot_01.IsOccupied` _asbp_base_poislot_01))
          (`KismetArrayLibrary.Array_Add` (`self.ValidSlots`) _asbp_base_poislot_01)))
      ;[1 1 1] Choose random POI Slot from array
      (`/Engine/EditorBlueprintResources/StandardMacros.IsValid` _item
        (:`Is Valid`
          (`BTFunctionLibrary.SetBlackboardValueAsObject` (`self.POISlot`) _item)
          (set `/Game/AICitizens/Blueprints/BP_BasePOISlot_01.OccupiedBy` OwnerActor _item)
          (`self.FinishExecute` true))
        (:`Is Not Valid`
          (`self.FinishExecute` false))))
    (:`CastFailed`
      (`self.FinishExecute` false))))