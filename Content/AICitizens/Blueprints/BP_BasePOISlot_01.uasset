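; Base point-of-interest slot for AI citizens that tracks its occupant and supplies an animation to play.
; On BeginPlay it totals the play chances of its animation list.
; GetAnimation uses that total for a weighted random pick, walking cumulative chances until one exceeds the roll.
; IsOccupied reports whether the OccupiedBy reference is valid.
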(event `self.ReceiveBeginPlay`
  (for _array_element (`self.AnimationToPlay`)
    (set `self.SummaryAnimationsChance` (+ (`.PlayChance_5_7D2E2EDC4EE307666EE9059956CF66A2` (break `/Game/AICitizens/Blueprints/SlotAnim` _array_element)) (`self.SummaryAnimationsChance`)))))

(fn `GetAnimation`
  (returns (Animation :type "AnimMontage Object Reference"))
  (locals (RandomChance :type "Float (double-precision)") (ActualChance :type "Float (double-precision)"))
  (set `local.RandomChance` (`KismetMathLibrary.RandomFloatInRange` 0.0 (`self.SummaryAnimationsChance`)))
  (for _array_element (`self.AnimationToPlay`)
    (bind _output_get (set `local.ActualChance` (+ (`.PlayChance_5_7D2E2EDC4EE307666EE9059956CF66A2` (break `/Game/AICitizens/Blueprints/SlotAnim` _array_element)) (`local.ActualChance`))))
    (if (> _output_get (`local.RandomChance`))
      (return (break `/Game/AICitizens/Blueprints/SlotAnim` _array_element))))
  (return null))

(fn `IsOccupied`
  (returns (Occupied :type Boolean))
  (return (`KismetSystemLibrary.IsValid` (`self.OccupiedBy`))))

(fn `UserConstructionScript`)