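; Base AI character for an AI test, with health, hit feedback and a treasure-scramble behavior.
; Tick turns its world widgets toward the camera, updating the health bar and the blackboard's current task name.
; Damage lowers health, plays a montage and flashes a dynamic material through a timeline.
; Scramble events toggle the FindTarget component and write behavior enums to the controller's blackboard, randomizing behavior when the scramble ends.
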(event `self.ReceiveBeginPlay`
  (bind _returnvalue (`GameplayStatics.GetPlayerController` 0))
  ;[1 1 1] 创建Ai状态测试UI
  (bind _returnvalue_2 (`|CreateWidget` "/Game/AiTest/AiStateWidget/AiStateWidget.AiStateWidget_C" _returnvalue))
  (set `self.AiState` _returnvalue_2)
  (bind _returnvalue_3 (`|CreateWidget` "/Game/Developers/17421/UMG/SkillUMG/Health.Health_C" _returnvalue))
  (set `self.HealthBar` _returnvalue_3)
  (`WidgetComponent.SetWidget` (`self.Widget`) (`self.AiState`))
  (`WidgetComponent.SetWidget` (`self.Widget1`) (`self.HealthBar`)))

(event `self.ReceiveTick`
  (params (DeltaSeconds :type "Float (single-precision)"))
  (bind _widget (`self.Widget`))
  (bind _returnvalue (`SceneComponent.K2_GetComponentLocation` (`PlayerCameraManager.TransformComponent` (`GameplayStatics.GetPlayerCameraManager` 0))))
  ;[1 1 1] 同步血条
  (set `/Game/Developers/17421/UMG/SkillUMG/Health.Health` (/ (`self.Health`) 100.0) (`self.HealthBar`))
  ;[1 1 1] Ai状态UI显示调整
  (`SceneComponent.K2_SetWorldRotation` _widget (`KismetMathLibrary.FindLookAtRotation` (`SceneComponent.K2_GetComponentLocation` _widget) _returnvalue) false false)
  (`SceneComponent.K2_SetWorldRotation` _widget (`KismetMathLibrary.FindLookAtRotation` (`SceneComponent.K2_GetComponentLocation` (`self.Widget1`)) _returnvalue) false false)
  (`SceneComponent.K2_SetWorldRotation` (`self.Widget1`) (`KismetMathLibrary.FindLookAtRotation` (`SceneComponent.K2_GetComponentLocation` (`self.Widget1`)) _returnvalue) false false)
  (bind _asbp_base_ai_controller (cast `/Game/AiTest/BP_BaseAiController` (`AIBlueprintHelperLibrary.GetAIController` self)))
  (`TextBlock.SetText` (`/Game/AiTest/AiStateWidget/AiStateWidget.State` (`self.AiState`)) (`KismetTextLibrary.Conv_StringToText` (`BlackboardComponent.GetValueAsString` (`/Game/AiTest/BP_BaseAiController.BTTBlackBoard` _asbp_base_ai_controller) "TaskName"))))

(event `self.ReceiveAnyDamage`
  (params (Damage :type "Float (single-precision)") (DamageType :type "DamageType Object Reference") (InstigatedBy :type "Controller Object Reference") (DamageCauser :type "Actor Object Reference"))
  (bind _mat (`self.Mat`))
  ;[1 1 1] 受到任何伤害处理血量
  (set `self.Health` (- (`self.Health`) Damage))
  ;[1 1 1] 受击动画
  (`self.PlayAnimMontage` "/Game/AiTest/Character/Animations/AM_Talking_02.AM_Talking_02")
  ;[1 1 1] 受击特效
  (`MaterialInstanceDynamic.SetVectorParameterValue` _mat "Color" (struct :`R` 0.109375 :`G` 0.060376 :`B` 0.03239 :`A` 1.0))
  (bind (_direction _vector) (`Timeline|闪烁` :!via `PlayFromStart`)
    (:`Update`
      (`MaterialInstanceDynamic.SetVectorParameterValue` _mat "BoneColor" (`KismetMathLibrary.Conv_VectorToLinearColor` _vector))
      (`MaterialInstanceDynamic.K2_GetVectorParameterValue` _mat "BoneColor"))
    (:`Finished`
      (`MaterialInstanceDynamic.SetVectorParameterValue` _mat "Color" (struct :`R` 1.0 :`G` 0.552012 :`B` 0.296138 :`A` 1.0))
      (set `self.AIControllerClass` "/Game/AiTest/BP_BaseAiController.BP_BaseAiController_C"))))

(event `ScrambleForTreasure`
  (`SceneComponent.SetVisibility` (`self.FindTarget`) true false)
  (bind _asbp_base_ai_controller (cast `/Game/AiTest/BP_BaseAiController` (`AIBlueprintHelperLibrary.GetAIController` self)))
  (bind _bttblackboard (`/Game/AiTest/BP_BaseAiController.BTTBlackBoard` _asbp_base_ai_controller))
  (`BlackboardComponent.SetValueAsEnum` _bttblackboard "BehaviorState" (`self.BehaviorState`))
  (`BlackboardComponent.SetValueAsEnum` _bttblackboard "CombatTaskState" (`self.CombatTask`)))

(event `EndOfScramble`
  (`SceneComponent.SetVisibility` (`self.FindTarget`) false false)
  (bind _asbp_base_ai_controller (cast `/Game/AiTest/BP_BaseAiController` (`AIBlueprintHelperLibrary.GetAIController` self)))
  (`BlackboardComponent.SetValueAsEnum` (`/Game/AiTest/BP_BaseAiController.BTTBlackBoard` _asbp_base_ai_controller) "BehaviorState" (`KismetMathLibrary.Conv_IntToByte` (`KismetMathLibrary.RandomIntegerInRange` 0 2))))

(fn `UserConstructionScript`
  (bind _returnvalue (`PrimitiveComponent.CreateDynamicMaterialInstance` (`self.Mesh`) 0 "/Game/AiTest/Mat_Base_Inst.Mat_Base_Inst" "None"))
  (set `self.Mat` _returnvalue))