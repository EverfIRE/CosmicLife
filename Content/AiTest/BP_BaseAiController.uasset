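; BP_BaseAiController is an AI controller that starts a pawn's behavior tree with randomized starting states.
; On BeginPlay it runs BT_MainTree, sets up the BT_MainBk blackboard and stores the blackboard component.
; It then writes a separate random value into the BehaviorState and RestState enum keys, each picked from three options.
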(event `self.ReceiveBeginPlay`
  (bind _bttblackboard (`self.BTTBlackBoard`))
  (`self.RunBehaviorTree` "/Game/AiTest/BT_MainTree.BT_MainTree")
  (bind _blackboardcomponent (`self.UseBlackboard` "/Game/AiTest/BT_MainBk.BT_MainBk"))
  (set `self.BTTBlackBoard` _blackboardcomponent)
  (`BlackboardComponent.SetValueAsEnum` _bttblackboard "BehaviorState" (`KismetMathLibrary.Conv_IntToByte` (`KismetMathLibrary.RandomIntegerInRange` 0 2)))
  (`BlackboardComponent.SetValueAsEnum` _bttblackboard "RestState" (`KismetMathLibrary.Conv_IntToByte` (`KismetMathLibrary.RandomIntegerInRange` 0 2))))

(fn `UserConstructionScript`)