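; BP_BaseAi_2 is a test AI actor that shows its current Behavior Tree state in a widget above it for debugging.
; On BeginPlay it creates an AiStateWidget and assigns it to its Widget component.
; Each Tick it rotates the widget to face the player camera and copies the TaskName string from the BP_BaseAiController2 blackboard into the widget's State text.
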(event `self.ReceiveBeginPlay`
  ;[1 1 1] 创建Ai状态测试UI
  (bind _returnvalue (`|CreateWidget` "/Game/AiTest/AiStateWidget/AiStateWidget.AiStateWidget_C" (`GameplayStatics.GetPlayerController` 0)))
  (bind _output_get (set `self.AiState` _returnvalue))
  (`WidgetComponent.SetWidget` (`self.Widget`) _output_get))

(event `self.ReceiveTick`
  (params (DeltaSeconds :type "Float (single-precision)"))
  (bind _widget (`self.Widget`))
  ;[1 1 1] Ai状态UI显示调整
  (`SceneComponent.K2_SetWorldRotation` _widget (`KismetMathLibrary.FindLookAtRotation` (`SceneComponent.K2_GetComponentLocation` _widget) (`SceneComponent.K2_GetComponentLocation` (`PlayerCameraManager.TransformComponent` (`GameplayStatics.GetPlayerCameraManager` 0)))) false false)
  (bind _asbp_base_ai_controller_2 (cast `/Game/AiTest/AiTreeTest/BP_BaseAiController2` (`AIBlueprintHelperLibrary.GetAIController` self)))
  (`TextBlock.SetText` (`/Game/AiTest/AiStateWidget/AiStateWidget.State` (`self.AiState`)) (`KismetTextLibrary.Conv_StringToText` (`BlackboardComponent.GetValueAsString` (`/Game/AiTest/AiTreeTest/BP_BaseAiController2.BTTBlackBoard` _asbp_base_ai_controller_2) "TaskName"))))

(fn `UserConstructionScript`)